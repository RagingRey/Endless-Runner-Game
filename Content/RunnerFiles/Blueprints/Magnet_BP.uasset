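; Magnet pickup actor for the runner game that temporarily activates the player character's magnet power.
; On overlap with BP_ThirdPersonCharacter, it sets IsMagnetActive on that character and hides its mesh.
; After a fixed delay it clears the flag on player pawn 0, prints status messages and destroys itself.
; Collision is not disabled while hidden, and the attraction effect itself is not implemented here.
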(event `self.ReceiveActorBeginOverlap`
  (params (OtherActor :type "Actor Object Reference"))
  (bind _asbp_third_person_character (cast `/Game/ThirdPerson/Blueprints/BP_ThirdPersonCharacter` OtherActor))
  (set `/Game/ThirdPerson/Blueprints/BP_ThirdPersonCharacter.IsMagnetActive` true _asbp_third_person_character)
  (`KismetSystemLibrary.PrintString` "Magnet Active")
  (`SceneComponent.SetVisibility` (`self.StaticMesh`) false false)
  (`KismetSystemLibrary.Delay` 10.0)
  (bind _asbp_third_person_character_2 (cast `/Game/ThirdPerson/Blueprints/BP_ThirdPersonCharacter` (`GameplayStatics.GetPlayerPawn` 0)))
  (set `/Game/ThirdPerson/Blueprints/BP_ThirdPersonCharacter.IsMagnetActive` false _asbp_third_person_character_2)
  (`KismetSystemLibrary.PrintString` "Magnet Inactive")
  (`self.K2_DestroyActor`))

(fn `UserConstructionScript`)