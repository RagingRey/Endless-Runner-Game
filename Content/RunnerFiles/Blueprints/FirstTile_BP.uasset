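; First floor tile of a lane-based endless runner, advancing the run as the player crosses it.
; BoxTrigger overlap makes the game mode spawn another tile, adds points, raises clamped walk speed, then destroys this tile after a delay.
; SpawnObstacles, not called here, randomly places pipes, boxes, coins, magnets or jumper boots across three lanes.
; Each check rerolls, and boots or an empty result skip remaining lanes.
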(event `self.ReceiveBeginPlay`)

(event `self.BoxTrigger.OnComponentBeginOverlap`
  (params (OverlappedComponent :type "PrimitiveComponent Object Reference") (OtherActor :type "Actor Object Reference") (OtherComp :type "PrimitiveComponent Object Reference") (OtherBodyIndex :type Integer) (bFromSweep :type Boolean) (SweepResult :type "HitResult Structure (by ref)"))
  (cast `/Game/ThirdPerson/Blueprints/BP_ThirdPersonCharacter` OtherActor)
  (bind _asbp_third_person_game_mode (cast `/Game/ThirdPerson/Blueprints/BP_ThirdPersonGameMode` (`GameplayStatics.GetGameMode`)))
  (`/Game/ThirdPerson/Blueprints/BP_ThirdPersonGameMode.SpawnTile` _asbp_third_person_game_mode)
  (bind _asbp_third_person_game_mode_2 (cast `/Game/ThirdPerson/Blueprints/BP_ThirdPersonGameMode` (`GameplayStatics.GetGameMode`)))
  (set `/Game/ThirdPerson/Blueprints/BP_ThirdPersonGameMode.CurrentPoints` (+ (`/Game/ThirdPerson/Blueprints/BP_ThirdPersonGameMode.PointsMultiplier` _asbp_third_person_game_mode_2) (`/Game/ThirdPerson/Blueprints/BP_ThirdPersonGameMode.CurrentPoints` _asbp_third_person_game_mode_2)) _asbp_third_person_game_mode_2)
  (bind _asbp_third_person_character (cast `/Game/ThirdPerson/Blueprints/BP_ThirdPersonCharacter` (`GameplayStatics.GetPlayerPawn` 0)))
  (bind _charactermovement (`Character.CharacterMovement` _asbp_third_person_character))
  (set `CharacterMovementComponent.MaxWalkSpeed` (`KismetMathLibrary.FClamp` (* (`CharacterMovementComponent.MaxWalkSpeed` _charactermovement) 1.01) 600.0 1800.0) _charactermovement)
  (`KismetSystemLibrary.Delay` 0.5)
  (`self.K2_DestroyActor`))

(fn `SpawnObstacles`
  (bind _returnvalue (`KismetMathLibrary.RandomFloatInRange` 0.0 1.0))
  (bind _returnvalue_2 (`KismetMathLibrary.RandomFloatInRange` 0.0 1.0))
  (bind _returnvalue_3 (`KismetMathLibrary.RandomFloatInRange` 0.0 1.0))
  (bind _returnvalue_4 (`SceneComponent.K2_GetComponentToWorld` (`self.LaneLeft`)))
  (bind _returnvalue_5 (`SceneComponent.K2_GetComponentToWorld` (`self.LaneMiddle`)))
  (bind _returnvalue_6 (`SceneComponent.K2_GetComponentToWorld` (`self.LaneRight`)))
  ;[1 1 1] Lane Left
  (if (`KismetMathLibrary.InRange_FloatFloat` _returnvalue_2 0.0 0.4)
    (`|SpawnActorFromClass` "/Game/RunnerFiles/Blueprints/Obstacle_Pipe_BP.Obstacle_Pipe_BP_C" _returnvalue_4 "Undefined" "OverrideRootScale" null null)
    ;[1 1 1] Lane Middle
    (if (`KismetMathLibrary.InRange_FloatFloat` _returnvalue_3 0.0 0.4) :!label _label
      (`|SpawnActorFromClass` "/Game/RunnerFiles/Blueprints/Obstacle_Pipe_BP.Obstacle_Pipe_BP_C" _returnvalue_5 "Undefined" "OverrideRootScale" null null)
      ;[1 1 1] Lane Right
      (if (`KismetMathLibrary.InRange_FloatFloat` _returnvalue 0.0 0.4) :!label _label_2
        (`|SpawnActorFromClass` "/Game/RunnerFiles/Blueprints/Obstacle_Pipe_BP.Obstacle_Pipe_BP_C" _returnvalue_6 "Undefined" "OverrideRootScale" null null)
        (elif (`KismetMathLibrary.InRange_FloatFloat` _returnvalue 0.4 0.5)
          (`|SpawnActorFromClass` "/Game/RunnerFiles/Blueprints/Obstacle_Box_BP.Obstacle_Box_BP_C" _returnvalue_6 "Undefined" "OverrideRootScale" null null)
          (elif (`KismetMathLibrary.InRange_FloatFloat` _returnvalue 0.5 0.95)
            (`|SpawnActorFromClass` "/Game/RunnerFiles/Blueprints/Coin_BP.Coin_BP_C" _returnvalue_6 "Undefined" "OverrideRootScale" null null)
            (elif (`KismetMathLibrary.InRange_FloatFloat` _returnvalue 0.95 0.975)
              (`|SpawnActorFromClass` "/Game/RunnerFiles/Blueprints/Magnet_BP.Magnet_BP_C" _returnvalue_6 "Undefined" "OverrideRootScale" null null)
              (elif (`KismetMathLibrary.InRange_FloatFloat` _returnvalue 0.975)
                (`|SpawnActorFromClass` "/Game/RunnerFiles/Blueprints/JumperBoots_BP.JumperBoots_BP_C" _returnvalue_6 "Undefined" "OverrideRootScale" null null))))))
      (elif (`KismetMathLibrary.InRange_FloatFloat` _returnvalue_3 0.4 0.5)
        (`|SpawnActorFromClass` "/Game/RunnerFiles/Blueprints/Obstacle_Box_BP.Obstacle_Box_BP_C" _returnvalue_5 "Undefined" "OverrideRootScale" null null)
        (goto _label_2)
        (elif (`KismetMathLibrary.InRange_FloatFloat` _returnvalue_3 0.5 0.95)
          (`|SpawnActorFromClass` "/Game/RunnerFiles/Blueprints/Coin_BP.Coin_BP_C" _returnvalue_5 "Undefined" "OverrideRootScale" null null)
          (goto _label_2)
          (elif (`KismetMathLibrary.InRange_FloatFloat` _returnvalue_3 0.95 0.975)
            (`|SpawnActorFromClass` "/Game/RunnerFiles/Blueprints/Magnet_BP.Magnet_BP_C" _returnvalue_5 "Undefined" "OverrideRootScale" null null)
            (goto _label_2)
            (elif (`KismetMathLibrary.InRange_FloatFloat` _returnvalue_3 0.975)
              (`|SpawnActorFromClass` "/Game/RunnerFiles/Blueprints/JumperBoots_BP.JumperBoots_BP_C" _returnvalue_5 "Undefined" "OverrideRootScale" null null))))))
    (elif (`KismetMathLibrary.InRange_FloatFloat` _returnvalue_2 0.4 0.5)
      (`|SpawnActorFromClass` "/Game/RunnerFiles/Blueprints/Obstacle_Box_BP.Obstacle_Box_BP_C" _returnvalue_4 "Undefined" "OverrideRootScale" null null)
      (goto _label)
      (elif (`KismetMathLibrary.InRange_FloatFloat` _returnvalue_2 0.5 0.95)
        (`|SpawnActorFromClass` "/Game/RunnerFiles/Blueprints/Coin_BP.Coin_BP_C" _returnvalue_4 "Undefined" "OverrideRootScale" null null)
        (goto _label)
        (elif (`KismetMathLibrary.InRange_FloatFloat` _returnvalue_2 0.95 0.975)
          (`|SpawnActorFromClass` "/Game/RunnerFiles/Blueprints/Magnet_BP.Magnet_BP_C" _returnvalue_4 "Undefined" "OverrideRootScale" null null)
          (goto _label)
          (elif (`KismetMathLibrary.InRange_FloatFloat` _returnvalue_2 0.975)
            (`|SpawnActorFromClass` "/Game/RunnerFiles/Blueprints/JumperBoots_BP.JumperBoots_BP_C" _returnvalue_4 "Undefined" "OverrideRootScale" null null)))))))

(fn `UserConstructionScript`)